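; BP_Water is a water surface actor that serves as either blue water or dead water, chosen by IsDeadWater.
; Its construction script sets the WaterUpper material's color and opacity per type.
; On authority, it seeds BP_MainGS with starting heights, then moves to that game state's height for its type each tick.
; Blue water stops ticking and hides WaterUpper once dead water rises above it.
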(event `self.ReceiveBeginPlay`
  (bind (_returnvalue_x _returnvalue_y _returnvalue_z) (`KismetMathLibrary.BreakVector` (`self.K2_GetActorLocation`)))
  ;[1 1 1] 초기화
  (`/Engine/EditorBlueprintResources/ActorMacros.Switch Has Authority`
    (:`Authority`
      (bind _asbp_main_gs (cast `/Game/Blueprints/System/Main/BP_MainGS` (`GameplayStatics.GetGameState`)))
      (if (`self.IsDeadWater`)
        (`/Game/Blueprints/System/Main/BP_MainGS.InitDeadWaterValues` _asbp_main_gs _returnvalue_z)
        (else
          (`/Game/Blueprints/System/Main/BP_MainGS.InitWaterValues` _asbp_main_gs _returnvalue_z (`self.FullZ`)))))))

(event `self.ReceiveTick`
  (params (DeltaSeconds :type "Float (single-precision)"))
  (bind (_returnvalue_x _returnvalue_y) (`KismetMathLibrary.BreakVector` (`self.K2_GetActorLocation`)))
  ;[1 1 1] Tick
  (`/Engine/EditorBlueprintResources/ActorMacros.Switch Has Authority`
    (:`Authority`
      (bind _asbp_main_gs (cast `/Game/Blueprints/System/Main/BP_MainGS` (`GameplayStatics.GetGameState`)))
      (bind _bluewaterheight (`/Game/Blueprints/System/Main/BP_MainGS.BlueWaterHeight` _asbp_main_gs))
      (bind _deadwaterheight (`/Game/Blueprints/System/Main/BP_MainGS.DeadWaterHeight` _asbp_main_gs))
      (`self.K2_SetActorLocation` (`KismetMathLibrary.MakeVector` _returnvalue_x _returnvalue_y (select `bool` (`self.IsDeadWater`) :`false` _bluewaterheight :`true` _deadwaterheight)))
      (if (and (not (`self.IsDeadWater`)) (> _deadwaterheight _bluewaterheight))
        (`self.DisableBluewater`)))))

(event `DisableBluewater`
  (`self.SetActorTickEnabled` false)
  (`/Engine/EditorBlueprintResources/StandardMacros.IsValid` self
    (:`Is Valid`
      (`SceneComponent.SetVisibility` (`self.WaterUpper`) false false)
      (`KismetSystemLibrary.PrintString` "Blue Water disable"))))

(fn `UserConstructionScript`
  (bind _waterupper (`self.WaterUpper`))
  (`MeshComponent.SetVectorParameterValueOnMaterials` _waterupper "WaterColor" (select `bool` (`self.IsDeadWater`) :`false` (`KismetMathLibrary.Conv_LinearColorToVector` (`self.BlueWaterColor`)) :`true` (`KismetMathLibrary.Conv_LinearColorToVector` (`self.DeadWaterColor`))))
  (`MeshComponent.SetScalarParameterValueOnMaterials` _waterupper "Opacity" (select `bool` (`self.IsDeadWater`) :`false` 0.9 :`true` 0.95 :!type "Float (single-precision)")))