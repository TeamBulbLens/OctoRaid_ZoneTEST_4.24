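; Spinning VR tutorial icon that shows only to the octopus player and is hidden, with collision off, for the hunter.
; When clickable, overlapping a motion controller activates it once, revealing its text widget, switching its color and playing a click sound.
; Until activated, external Highlight calls apply the GameInstance's highlight color, and Tick clears it through a flag once those calls stop.
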(event `self.Highlight`
  ;[1 1 1] Highlight
  (if (`self.Clickable`)
    (if (not (`self.Activated`))
      (`MeshComponent.SetVectorParameterValueOnMaterials` (`self.Icon`) "HighlightColor" (`KismetMathLibrary.Conv_LinearColorToVector` (`self.HighlightColor`)))
      (set `self.IsHighlighted` true))))

(event `self.Highlight_Back`
  ;[1 1 1] Highlight
  (if (`self.Clickable`)
    (`MeshComponent.SetVectorParameterValueOnMaterials` (`self.Icon`) "HighlightColor" (0.0 0.0 0.0))))

(event `self.ReceiveBeginPlay`
  ;[1 1 1] 로컬 플레이어가 헌터면 아이콘을 숨기고, 문어면 텍스트 설정
  (`SceneComponent.SetVisibility` (`self.Widget`) false false)
  (cast `/Game/Blueprints/Octopus/BP_VRPawnMain` (`Controller.K2_GetPawn` (`GameplayStatics.GetPlayerController` 0))
    (:`then`
      (`SceneComponent.SetVisibility` (`self.Widget`) (`self.Activated`) false)
      (bind _asvrtutorial_text (cast `/Game/Blueprints/Public/TutorialIcons/VRTutorialText` (`WidgetComponent.GetUserWidgetObject` (`self.Widget`))))
      (`/Game/Blueprints/Public/TutorialIcons/VRTutorialText.SetText` _asvrtutorial_text (`self.Text`))
      (`MeshComponent.SetScalarParameterValueOnMaterials` (`self.Icon`) "Color" (select `/Game/Blueprints/Public/3DButton/IconColor_Enum` (`self.DefalutColor`) :`NewEnumerator0` 0.01 :`NewEnumerator1` 0.1 :`NewEnumerator2` 0.2 :`NewEnumerator3` 0.3 :`NewEnumerator4` 0.4 :`NewEnumerator10` 0.5 :`NewEnumerator5` 0.6 :`NewEnumerator6` 0.7 :`NewEnumerator9` 1.0 :!type "Float (single-precision)")))
    (:`CastFailed`
      (`SceneComponent.SetVisibility` (`self.Icon`) false false)
      (`PrimitiveComponent.SetCollisionEnabled` (`self.Box`) "NoCollision"))))

(event `self.Box.OnComponentBeginOverlap`
  (params (OverlappedComponent :type "PrimitiveComponent Object Reference") (OtherActor :type "Actor Object Reference") (OtherComp :type "PrimitiveComponent Object Reference") (OtherBodyIndex :type Integer) (bFromSweep :type Boolean) (SweepResult :type "HitResult Structure (by ref)"))
  ;[1 1 1] 겹쳐지면 텍스트 띄우기
  (if (`self.Clickable`)
    (cast `/Game/Blueprints/Octopus/BP_MotionControllerMain` OtherActor)
    (if (not (`self.Activated`))
      (set `self.Activated` true)
      (`self.Highlight_Back`)
      (`SceneComponent.SetVisibility` (`self.Widget`) true false)
      (`MeshComponent.SetScalarParameterValueOnMaterials` (`self.Icon`) "Color" (select `/Game/Blueprints/Public/3DButton/IconColor_Enum` (`self.SelectedColor`) :`NewEnumerator0` 0.01 :`NewEnumerator1` 0.1 :`NewEnumerator2` 0.2 :`NewEnumerator3` 0.3 :`NewEnumerator4` 0.4 :`NewEnumerator10` 0.5 :`NewEnumerator5` 0.6 :`NewEnumerator6` 0.7 :`NewEnumerator9` 1.0 :!type "Float (single-precision)"))
      (`GameplayStatics.SpawnSoundAtLocation` "/Game/Resources/Ultimate_SFX_Bundle/Casual_Bundle/UI_Item_Sounds/Cues/8_Bit_click_sounds/8_Bit_click_sounds_7_Cue.8_Bit_click_sounds_7_Cue" (`SceneComponent.K2_GetComponentLocation` (`self.Icon`)) (struct) 1.0 1.0 0.0 null null))))

(event `self.ReceiveTick`
  (params (DeltaSeconds :type "Float (single-precision)"))
  ;[1 1 1] highlight 상태 업데이트
  (`|ExecutionSequence`
    (:`then_0`
      (if (`self.Clickable`)
        (if (`self.Activated`)
          _
          (elif (`self.IsHighlighted`)
            (set `self.IsHighlighted` false)
            (else
              (`self.Highlight_Back`))))))
    (:`then_1`
      (`SceneComponent.K2_AddLocalRotation` (`self.Icon`) (* (struct :`Yaw` 200.0) (`GameplayStatics.GetWorldDeltaSeconds`)) false false))))

(fn `UserConstructionScript`
  (bind _asbp_gi (cast `/Game/Blueprints/Public/BP_GI` (`GameplayStatics.GetGameInstance`)))
  (set `self.HighlightColor` (`/Game/Blueprints/Public/BP_GI.OctoHighlightColor` _asbp_gi)))