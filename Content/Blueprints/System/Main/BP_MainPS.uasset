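; Main PlayerState for Hunters and the VR Octopus, holding role, HP, UID and skin.
; Pushes GameInstance UID/skin to the server, requests new info for mid-game joiners, then spawns or skins Hunters, whose input unlocks after skinning.
; Server Tick applies water effects during play: both waters damage Hunters, while Blue Water heals and Dead Water harms the Octopus, whose underwater display also updates.
; CurrentHP's RepNotify refreshes Hunter HUD and billboard HP bars.
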(event `SetLocalInfoServer`
  ;[1 1 1] 헌터 초기 세팅
  ;;[1 1 1] 각각의 클라이언트가 각각의 GameInstance에 저장되어있는 UID와 Skin을 새로생긴 PlayerState에 넣으라고 지시
  (`KismetSystemLibrary.Delay` 2.0)
  (bind _outactors (`GameplayStatics.GetAllActorsOfClass` "BP_MainPS_C"))
  (for _array_element _outactors
    (`self.SetLocalInfo` _array_element)))

(event `SetUIDAndSkinServer`
  (params (PlayerState :type "/Game/Blueprints/System/Main/BP_MainPS Object Reference"))
  ;[1 1 1] 헌터 초기 세팅
  ;;[1 1 1] 중간난입자를 위한 세팅
  ;;;[1 1 1] 서버에 비어있는 UID와 Skin을 요청
  (bind _asbp_main_gm (cast `/Game/Blueprints/System/Main/BP_MainGM` (`GameplayStatics.GetGameMode`)))
  (`/Engine/EditorBlueprintResources/StandardMacros.IsValid` _asbp_main_gm
    (:`Is Valid`
      (`/Game/Blueprints/System/Main/BP_MainGM.SetNewClientUserInfo` _asbp_main_gm PlayerState))))

(event `SetLocalInfo`
  ;[1 1 1] 헌터 초기 세팅
  (bind _asbp_gi (cast `/Game/Blueprints/Public/BP_GI` (`GameplayStatics.GetGameInstance`)))
  (`/Engine/EditorBlueprintResources/StandardMacros.IsValid` _asbp_gi
    (:`Is Valid`
      (bind _localuid (`/Game/Blueprints/Public/BP_GI.LocalUID` _asbp_gi))
      (if (== _localuid -1)
        ;;[1 1 1] 이 시점에서 Local UID 가 -1이면 중간 난입임 아예 세팅을 새로 해주자
        (`self.SetUIDAndSkinServer` self)
        (elif (not (`self.InfoIsSet`))
          (`self.SetUIDServer` _localuid)
          (bind _localskinstate (`/Game/Blueprints/Public/BP_GI.LocalSkinState` _asbp_gi))
          (`self.SetSkinStateServer` _localskinstate)
          (set `self.UID` _localuid)
          (set `self.SkinState` _localskinstate)
          (set `self.InfoIsSet` true)
          (`self.InitHP`)
          (`/Engine/EditorBlueprintResources/StandardMacros.IsValid` (`GameplayStatics.GetGameMode`)
            (:`Is Not Valid`
              ;;[1 1 1] 플레이어폰이 없으면 스폰
              (bind _asbp_player_character_sn (cast `/Game/Blueprints/SN/Blueprints_SN/BP_PlayerCharacter_SN` (`self.PawnPrivate`))
                (:`then`
                  ;;[1 1 1] 스폰되어있으면 스킨 세팅
                  (`/Engine/EditorBlueprintResources/StandardMacros.IsValid` _asbp_player_character_sn
                    (:`Is Valid`
                      (bind _asbp_main_pc (cast `/Game/Blueprints/System/Main/BP_MainPC` (`self.GetOwner`)))
                      (`/Engine/EditorBlueprintResources/StandardMacros.IsValid` _asbp_main_pc
                        (:`Is Valid`
                          (`/Game/Blueprints/System/Main/BP_MainPC.SetMeshAndMaterialAllPlayersServer` _asbp_main_pc))))))
                (:`CastFailed`
                  (`self.SpawnHunter`))))))))))

(event `SetLocalInfoToClientGI`
  (params (UID :type Integer) (SkinState :type "/Game/Blueprints/Skin/ESkinState Enum" :default "NewEnumerator0"))
  ;[1 1 1] 헌터 초기 세팅
  ;;[1 1 1] 중간난입자를 위한 세팅
  ;;;[1 1 1] 서버에서 받은 UID와 Skin을 클라이언트 GI에 저장
  (`/Engine/EditorBlueprintResources/StandardMacros.IsValid` (`GameplayStatics.GetGameMode`)
    (:`Is Not Valid`
      (bind _asbp_gi (cast `/Game/Blueprints/Public/BP_GI` (`GameplayStatics.GetGameInstance`)))
      (`/Engine/EditorBlueprintResources/StandardMacros.IsValid` _asbp_gi
        (:`Is Valid`
          (`/Game/Blueprints/Public/BP_GI.SetLocalUID` _asbp_gi UID)
          (set `/Game/Blueprints/Public/BP_GI.LocalSkinState` SkinState _asbp_gi))))))

(event `self.ReceiveBeginPlay`
  ;[1 1 1] Init
  (`self.SetRoleState`)
  (`self.InitHP`)
  (if (`|EnumEquality` (`self.RoleState`) "NewEnumerator1")
    ;[1 1 1] 스폰시 입력막음
    (bind _asbp_main_pc (cast `/Game/Blueprints/System/Main/BP_MainPC` (`self.GetOwner`)))
    (`WidgetBlueprintLibrary.SetInputMode_UIOnlyEx` _asbp_main_pc null)))

(event `SpawnHunter`
  ;[1 1 1] 헌터 초기 세팅
  ;;[1 1 1] 헌터 스폰
  (bind _asbp_main_gm (cast `/Game/Blueprints/System/Main/BP_MainGM` (`GameplayStatics.GetGameMode`)))
  (`/Engine/EditorBlueprintResources/StandardMacros.IsValid` _asbp_main_gm
    (:`Is Valid`
      (bind _asbp_main_pc (cast `/Game/Blueprints/System/Main/BP_MainPC` (`self.GetOwner`)))
      (`/Engine/EditorBlueprintResources/StandardMacros.IsValid` _asbp_main_pc
        (:`Is Valid`
          (`/Game/Blueprints/System/Main/BP_MainGM.SpawnHunter` _asbp_main_gm _asbp_main_pc))))))

(event `SetUIDServer`
  (params (UID :type Integer))
  ;[1 1 1] 헌터 초기 세팅
  (set `self.UID` UID))

(event `self.ReceiveTick`
  (params (DeltaSeconds :type "Float (single-precision)"))
  (bind (_returnvalue_x _returnvalue_y _returnvalue_z) (`KismetMathLibrary.BreakVector` (`self.K2_GetActorLocation` (`self.PawnPrivate`))))
  (bind (_returnvalue_x_2 _returnvalue_y_2 _returnvalue_z_2) (`KismetMathLibrary.BreakVector` (`self.K2_GetActorLocation` (`self.PawnPrivate`))))
  (bind (_returnvalue_x_3 _returnvalue_y_3 _returnvalue_z_3) (`KismetMathLibrary.BreakVector` (`self.K2_GetActorLocation` (`self.PawnPrivate`))))
  ;[1 1 1] Tick
  (`/Engine/EditorBlueprintResources/StandardMacros.IsValid` (`GameplayStatics.GetGameMode`)
    (:`Is Valid`
      (`/Engine/EditorBlueprintResources/StandardMacros.IsValid` (`self.PawnPrivate`)
        (:`Is Valid`
          (bind _asbp_main_gs (cast `/Game/Blueprints/System/Main/BP_MainGS` (`GameplayStatics.GetGameState`)))
          (`|ExecutionSequence`
            (:`then_0`
              (if (`|EnumEquality` (`MainGS.CurrentGameState` _asbp_main_gs) "Playing")
                (if (> (`self.CurrentHP`) 0.0)
                  (bind _asbp_vrpawn_main (cast `/Game/Blueprints/Octopus/BP_VRPawnMain` (`self.PawnPrivate`))
                    (:`then`
                      (bind _returnvalue (`self.CheckHeight` _asbp_vrpawn_main (`/Game/Blueprints/System/Main/BP_MainGS.DeadWaterHeight` _asbp_main_gs)))
                      (if (or (`self.CheckHeight` _asbp_vrpawn_main (`/Game/Blueprints/System/Main/BP_MainGS.BlueWaterHeight` _asbp_main_gs)) _returnvalue)
                        (if _returnvalue
                          (`self.DamageByWater` DeltaSeconds true)
                          (else
                            (`self.HealingByWater` DeltaSeconds)))))
                    (:`CastFailed`
                      (bind _deadwaterheight (`/Game/Blueprints/System/Main/BP_MainGS.DeadWaterHeight` _asbp_main_gs))
                      (if (or (> (`/Game/Blueprints/System/Main/BP_MainGS.BlueWaterHeight` _asbp_main_gs) _returnvalue_z_2) (> _deadwaterheight _returnvalue_z_3))
                        (`self.DamageByWater` DeltaSeconds (> _deadwaterheight _returnvalue_z))))))))
            (:`then_1`
              (bind _asbp_vrpawn_main_2 (cast `/Game/Blueprints/Octopus/BP_VRPawnMain` (`self.PawnPrivate`)))
              (bind (_returnvalue_x_4 _returnvalue_y_4 _returnvalue_z_4) (`KismetMathLibrary.BreakVector` (`SceneComponent.K2_GetComponentLocation` (`/Game/Blueprints/Octopus/BP_VRPawnMain.Camera` _asbp_vrpawn_main_2))))
              (bind _returnvalue_2 (> (`/Game/Blueprints/System/Main/BP_MainGS.DeadWaterHeight` _asbp_main_gs) (- _returnvalue_z_4 200.0)))
              (`/Game/Blueprints/Octopus/BP_VRPawnMain.SetWaterState` _asbp_vrpawn_main_2 _returnvalue_2)
              (bind (_returnvalue_x_5 _returnvalue_y_5 _returnvalue_z_5) (`KismetMathLibrary.BreakVector` (`SceneComponent.K2_GetComponentLocation` (`/Game/Blueprints/Octopus/BP_VRPawnMain.Camera` _asbp_vrpawn_main_2))))
              (`/Game/Blueprints/Octopus/BP_VRPawnMain.ToggleUnderWaterWidget` _asbp_vrpawn_main_2 (or _returnvalue_2 (> (`/Game/Blueprints/System/Main/BP_MainGS.BlueWaterHeight` _asbp_main_gs) (- _returnvalue_z_5 200.0)))))))))))

(event `SetSkinStateServer`
  (params (SkinState :type "/Game/Blueprints/Skin/ESkinState Enum" :default "NewEnumerator0"))
  ;[1 1 1] 헌터 초기 세팅
  (set `self.SkinState` SkinState))

(event `SetMeshAndMaterial`
  ;[1 1 1] 헌터 초기 세팅
  (bind _asbp_player_character_sn (cast `/Game/Blueprints/SN/Blueprints_SN/BP_PlayerCharacter_SN` (`self.PawnPrivate`)))
  (`/Engine/EditorBlueprintResources/StandardMacros.IsValid` _asbp_player_character_sn
    (:`Is Valid`
      (bind _result (`/Game/Blueprints/Skin/BP_SkinData.GetSkinStruct` (`self.BP_SkinData`) (`self.SkinState`)))
      (bind _mesh (`Character.Mesh` _asbp_player_character_sn))
      (bind (_skin _mesh_2 _mat _portrait _helmetcolor) (break `/Game/Blueprints/Skin/SkinStruct` _result))
      (`SkinnedMeshComponent.SetSkinnedAssetAndUpdate` _mesh _mesh_2 true)
      (`PrimitiveComponent.SetMaterial` _mesh 0 _mat)
      (`PrimitiveComponent.SetMaterial` (`/Game/Blueprints/SN/Blueprints_SN/BP_PlayerCharacter_SN.Helmet` _asbp_player_character_sn) 0 _helmetcolor)
      (`self.InitHP`)
      ;;[1 1 1] 스킨 세팅후 조작가능하게
      (bind _asbp_main_pc (cast `/Game/Blueprints/System/Main/BP_MainPC` (`self.GetOwner`)))
      (`WidgetBlueprintLibrary.SetInputMode_GameOnly` _asbp_main_pc)
      (`KismetSystemLibrary.Delay` 0.2)
      (`/Game/Blueprints/SN/Blueprints_SN/BP_PlayerCharacter_SN.WeaponAttachment` _asbp_player_character_sn))))

(event `DamageByWater`
  (params (DeltaSeconds :type "Float (double-precision)") (IsDeadWater :type Boolean))
  ;[1 1 1] 헌터의 경우 물 데미지
  (bind _asbp_main_gs (cast `/Game/Blueprints/System/Main/BP_MainGS` (`GameplayStatics.GetGameState`)))
  (`GameplayStatics.ApplyDamage` (`self.PawnPrivate`) (* DeltaSeconds (select `bool` IsDeadWater :`false` (`/Game/Blueprints/System/Main/BP_MainGS.BlueWaterDamage` _asbp_main_gs) :`true` (`/Game/Blueprints/System/Main/BP_MainGS.DeadWaterDamage` _asbp_main_gs))) null null "/Game/Blueprints/Octopus/DamageType_Water.DamageType_Water_C"))

(event `HealingByWater`
  (params (DeltaSeconds :type "Float (double-precision)"))
  ;[1 1 1] 문어의 경우 회복
  (bind _asbp_main_gs (cast `/Game/Blueprints/System/Main/BP_MainGS` (`GameplayStatics.GetGameState`)))
  (`GameplayStatics.ApplyDamage` (`self.PawnPrivate`) (* DeltaSeconds -1.0 (`/Game/Blueprints/System/Main/BP_MainGS.BlueWaterHealing` _asbp_main_gs))))

(fn `GetMaxHP`
  (returns (MaxHP :type "Float (double-precision)"))
  (switch `/Game/Blueprints/Public/ERoleState` (`self.RoleState`)
    (:`NewEnumerator0`
      (return (`self.OctoMaxHP`)))
    (:`NewEnumerator1`
      (return (`self.HunterMaxHP`)))))

(fn `InitHP`
  (bind _maxhp (`self.GetMaxHP`))
  (set `self.CurrentHP` _maxhp))

(fn `IsAlive`
  (returns (IsAlive :type Boolean))
  (return (> (`self.CurrentHP`) 0.0)))

(fn `IsUnderWater`
  (returns (IsUnderWater :type Boolean) (IsUnderDeadWater :type Boolean))
  (bind _pawnprivate (`self.PawnPrivate`))
  (bind (_returnvalue_x _returnvalue_y _returnvalue_z) (`KismetMathLibrary.BreakVector` (`self.K2_GetActorLocation` _pawnprivate)))
  (bind _asbp_main_gs (cast `/Game/Blueprints/System/Main/BP_MainGS` (`GameplayStatics.GetGameState`)))
  (`/Engine/EditorBlueprintResources/StandardMacros.IsValid` _asbp_main_gs
    (:`Is Valid`
      (`/Engine/EditorBlueprintResources/StandardMacros.IsValid` _pawnprivate
        (:`Is Valid`
          (return (> (`/Game/Blueprints/System/Main/BP_MainGS.BlueWaterHeight` _asbp_main_gs) _returnvalue_z) (> (`/Game/Blueprints/System/Main/BP_MainGS.DeadWaterHeight` _asbp_main_gs) _returnvalue_z)))))))

(fn `OnHealingHP`
  (params (Healing :type "Float (double-precision)"))
  (bind _returnvalue (- (`self.CurrentHP`) Healing))
  (if (> _returnvalue (`self.OctoMaxHP`))
    (set `self.CurrentHP` (`self.OctoMaxHP`))
    (else
      (set `self.CurrentHP` _returnvalue))))

(fn `OnRep_CurrentHP`
  (bind _asbp_main_pc (cast `/Game/Blueprints/System/Main/BP_MainPC` (`self.GetOwner`)))
  (`/Engine/EditorBlueprintResources/StandardMacros.IsValid` _asbp_main_pc
    (:`Is Valid`
      (`/Game/Blueprints/System/Main/BP_MainPC.UpdateHunterMainWidgetServer` _asbp_main_pc)
      (bind _asbp_player_character_sn (cast `/Game/Blueprints/SN/Blueprints_SN/BP_PlayerCharacter_SN` (`self.PawnPrivate`)))
      (`/Engine/EditorBlueprintResources/StandardMacros.IsValid` _asbp_player_character_sn
        (:`Is Valid`
          (bind _ashunter_billboard_hpbar (cast `/Game/Blueprints/HunterUI/HunterBillboardHPBar` (`/Game/Blueprints/SN/Blueprints_SN/BP_PlayerCharacter_SN.BillboardWidget` _asbp_player_character_sn)))
          (`/Engine/EditorBlueprintResources/StandardMacros.IsValid` _ashunter_billboard_hpbar
            (:`Is Valid`
              (bind _maxhp (`self.GetMaxHP`))
              (`/Game/Blueprints/HunterUI/HunterBillboardHPBar.SetHPBarPercent` _ashunter_billboard_hpbar (/ (`self.CurrentHP`) _maxhp)))))))))

(fn `OnTakeDamage`
  (params (Damage :type "Float (double-precision)"))
  (bind _returnvalue (- (`self.CurrentHP`) Damage))
  (if (> _returnvalue 0.0)
    (bind _maxhp (`self.GetMaxHP`))
    (if (<= _returnvalue _maxhp)
      (set `self.CurrentHP` _returnvalue)
      (else
        (set `self.CurrentHP` _maxhp)))
    (else
      (set `self.CurrentHP` 0.0))))

(fn `SetInfo`
  (bind _asbp_main_pc (cast `/Game/Blueprints/System/Main/BP_MainPC` (`self.GetOwner`)))
  (`/Engine/EditorBlueprintResources/StandardMacros.IsValid` _asbp_main_pc
    (:`Is Valid`
      (if (`Controller.IsLocalPlayerController` _asbp_main_pc)
        (bind _asbp_gi (cast `/Game/Blueprints/Public/BP_GI` (`GameplayStatics.GetGameInstance`)))
        (`/Engine/EditorBlueprintResources/StandardMacros.IsValid` _asbp_gi
          (:`Is Valid`
            (bind _localuid (`/Game/Blueprints/Public/BP_GI.LocalUID` _asbp_gi))
            (if (not (== _localuid -1))
              (set `self.UID` _localuid)
              (set `self.SkinState` (`/Game/Blueprints/Public/BP_GI.LocalSkinState` _asbp_gi))
              (`self.SetMeshAndMaterial`))))
        (else
          (`self.SetLocalInfoServer`))))))

(fn `SetRoleState`
  (returns (IsOctopus :type Boolean))
  (bind _asbp_main_pc (cast `/Game/Blueprints/System/Main/BP_MainPC` (`self.GetOwner`)))
  (`/Engine/EditorBlueprintResources/StandardMacros.IsValid` _asbp_main_pc
    (:`Is Valid`
      (bind _output_get (set `self.RoleState` (`/Game/Blueprints/System/Main/BP_MainPC.RoleState` _asbp_main_pc)))
      (return (`|EnumEquality` _output_get "NewEnumerator0")))))

(fn `UserConstructionScript`
  (bind _asbp_main_pc (cast `/Game/Blueprints/System/Main/BP_MainPC` (`self.GetOwner`)))
  (`/Engine/EditorBlueprintResources/StandardMacros.IsValid` _asbp_main_pc
    (:`Is Valid`
      (if (`Controller.IsLocalPlayerController` _asbp_main_pc)
        _))))