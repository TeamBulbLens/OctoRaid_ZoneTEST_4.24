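; A character that VR motion controllers can grab, carry and throw, highlighted while it is a controller's grip target.
; Tick polls overlapping controllers for selection and auto-drops it when attached but not in use.
; Pickup attaches it and disables movement; Drop switches the capsule to physics, optionally adding throw velocity.
; After a delay, Server/Multicast event chains, gated by GameMode checks, stop physics and restore upright rotation and walking.
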(event `self.ReceiveBeginPlay`
  ;[1 1 1] BeginPlay
  (set `self.Origin_ActorCollisionRotator` (`SceneComponent.K2_GetComponentRotation` (`self.CapsuleComponent`)))
  (set `self.OriginActorRotation` (`SceneComponent.K2_GetComponentRotation` (`self.Mesh`))))

(event `/Game/Blueprints/BuildingsAndProps/Interactable_Interface.Highlight`
  (bind _mesh (`self.Mesh`))
  ;[1 1 1] highlight
  (cast `/Game/Blueprints/Octopus/BP_VRPawnMain` (`GameplayStatics.GetPlayerPawn` 0))
  (`MeshComponent.SetVectorParameterValueOnMaterials` _mesh "HighlightColor" (select `bool` (`self.IsUsing`) :`false` (`KismetMathLibrary.Conv_LinearColorToVector` (`self.SelectedColor`)) :`true` (`KismetMathLibrary.Conv_LinearColorToVector` (`self.UsingColor`))))
  (`MeshComponent.SetScalarParameterValueOnMaterials` _mesh "Intensity" 1.0)
  (set `self.IsHighlighted` true))

(event `/Game/Blueprints/BuildingsAndProps/Interactable_Interface.Highlight_Back`
  (bind _mesh (`self.Mesh`))
  ;[1 1 1] highlight
  (cast `/Game/Blueprints/Octopus/BP_VRPawnMain` (`GameplayStatics.GetPlayerPawn` 0))
  (`MeshComponent.SetVectorParameterValueOnMaterials` _mesh "HighlightColor" (0.0 0.0 0.0))
  (`MeshComponent.SetScalarParameterValueOnMaterials` _mesh "Intensity" 0.0))

(event `self.ReceiveTick`
  (params (DeltaSeconds :type "Float (single-precision)"))
  ;[1 1 1] 컨트롤러가 잡으려고 할 때 하이라이트 / 아니면 원래대로
  (`self.SelectStateUpdate`)
  (`self.HighlightStateUpdate`)
  (if (not (`self.IsUsing`))
    (`/Engine/EditorBlueprintResources/StandardMacros.IsValid` (`self.GetParentComponent`)
      (:`Is Valid`
        (`/Game/Blueprints/BuildingsAndProps/Pickup/PickupActorInterface.Drop` null)))))

(event `/Game/Blueprints/BuildingsAndProps/Pickup/PickupActorInterface.Pickup`
  (params (AttachTo :type "SceneComponent Object Reference"))
  ;[1 1 1] Pickup
  (`SceneComponent.K2_AttachToComponent` (`self.RootComponent`) AttachTo "None" "KeepWorld" "KeepWorld" "KeepWorld" false)
  (`CharacterMovementComponent.DisableMovement` (`self.CharacterMovement`))
  (set `self.IsUsing` true)
  (`KismetSystemLibrary.PrintString` (`KismetStringLibrary.Conv_BoolToString` (`self.IsDropped`)) true true (struct :`G` 0.66 :`B` 1.0 :`A` 1.0) 5.0))

(event `/Game/Blueprints/BuildingsAndProps/Pickup/PickupActorInterface.Drop`
  (params (Hand :type "SceneComponent Object Reference") (LinearVelocity :type "Vector Structure") (AngularVelocity :type "Vector Structure") (Fire :type Boolean))
  ;[1 1 1] Pickup
  (`/Engine/EditorBlueprintResources/StandardMacros.IsValid` (`GameplayStatics.GetGameMode`)
    (:`Is Valid`
      (`self.DropServer` LinearVelocity AngularVelocity Fire))))

(event `DropMulticast`
  ;[1 1 1] Pickup
  (`self.K2_DetachFromActor` "KeepWorld" "KeepWorld" "KeepWorld")
  (set `self.IsDropped` true)
  (set `self.IsUsing` false)
  (`KismetSystemLibrary.PrintString` (`KismetStringLibrary.Conv_BoolToString` (`self.IsDropped`)) true true (struct :`R` 1.0 :`B` 0.154543 :`A` 1.0) 5.0)
  (`self.Dropped`))

(event `DropServer`
  (params (NewVel :type "Vector Structure") (NewAngVel :type "Vector Structure") (Condition :type Boolean))
  (bind _capsulecomponent (`self.CapsuleComponent`))
  ;[1 1 1] Pickup
  (`PrimitiveComponent.SetSimulatePhysics` _capsulecomponent true)
  (if Condition
    (`PrimitiveComponent.SetPhysicsLinearVelocity` _capsulecomponent NewVel true "None")
    (`PrimitiveComponent.SetPhysicsAngularVelocityInDegrees` _capsulecomponent NewAngVel true "None"))
  (`self.DropMulticast`))

(event `self.CapsuleComponent.OnComponentHit`
  (params (HitComponent :type "PrimitiveComponent Object Reference") (OtherActor :type "Actor Object Reference") (OtherComp :type "PrimitiveComponent Object Reference") (NormalImpulse :type "Vector Structure") (Hit :type "HitResult Structure (by ref)"))
  ;[1 1 1] Dropped
  (if (`|EnumEquality` (`CharacterMovementComponent.MovementMode` (`self.CharacterMovement`)) "MOVE_None")
    (`/Engine/EditorBlueprintResources/StandardMacros.DoOnce` false :!label _label
      (:`Completed`
        (`self.Dropped`)
        (`KismetSystemLibrary.Delay` 3.0)
        (goto _label :!via `Reset`)))))

(event `self.ToPlayerGrabCollision.OnComponentBeginOverlap`
  (params (OverlappedComponent :type "PrimitiveComponent Object Reference") (OtherActor :type "Actor Object Reference") (OtherComp :type "PrimitiveComponent Object Reference") (OtherBodyIndex :type Integer) (bFromSweep :type Boolean) (SweepResult :type "HitResult Structure (by ref)"))
  ;[1 1 1] Dropped
  (if (`|EnumEquality` (`PrimitiveComponent.GetCollisionObjectType` OtherComp) "ECC_GameTraceChannel6")
    (`self.Dropped`)))

(event `Dropped`
  ;[1 1 1] Dropped
  (if (`self.IsDropped`)
    (`KismetSystemLibrary.Delay` 2.0)
    (`/Engine/EditorBlueprintResources/StandardMacros.IsValid` (`GameplayStatics.GetGameMode`)
      (:`Is Valid`
        (`self.DroppedServer`)))))

(event `DroppedServer`
  ;[1 1 1] Dropped
  (`self.DroppedMulticast`))

(event `DroppedMulticast`
  ;[1 1 1] Dropped
  (`PrimitiveComponent.SetSimulatePhysics` (`self.CapsuleComponent`) false)
  (set `self.IsDropped` false)
  (`self.RevertPlayerRotationServer`))

(event `RevertPlayerRotationServer`
  ;[1 1 1] Dropped
  (`self.RevertPlayerRotation`))

(event `RevertPlayerRotation`
  ;[1 1 1] Dropped
  (`SceneComponent.K2_SetWorldRotation` (`self.CapsuleComponent`) (`self.Origin_ActorCollisionRotator`) false false)
  (`CharacterMovementComponent.SetMovementMode` (`self.CharacterMovement`) "MOVE_Walking" 0)
  (`self.ClientRevertRotationServer`))

(event `ClientRevertRotation`
  ;[1 1 1] Dropped
  (`SceneComponent.K2_SetWorldRotation` (`self.CapsuleComponent`) (`self.Origin_ActorCollisionRotator`) false false))

(event `ClientRevertRotationServer`
  ;[1 1 1] Dropped
  (`self.ClientRevertRotation`))

(event `SetPhysicsOff`
  (`PrimitiveComponent.SetSimulatePhysics` (`self.CapsuleComponent`) false))

(event `Key|Nine`
  (params (Key :type "Key Structure"))
  (:`Pressed`
    (bind _asbp_gi (cast `/Game/Blueprints/Public/BP_GI` (`GameplayStatics.GetGameInstance`)))
    (if (`/Game/Blueprints/Public/BP_GI.IsDebugMode` _asbp_gi)
      (`PrimitiveComponent.SetSimulatePhysics` (`self.CapsuleComponent`) false)
      (`self.ClientRevertRotationServer`))))

(event `Key|Zero`
  (params (Key :type "Key Structure"))
  (:`Pressed`
    (bind _asbp_gi (cast `/Game/Blueprints/Public/BP_GI` (`GameplayStatics.GetGameInstance`)))
    (if (`/Game/Blueprints/Public/BP_GI.IsDebugMode` _asbp_gi)
      (`PrimitiveComponent.SetSimulatePhysics` (`self.CapsuleComponent`) true))))

(fn `HighlightStateUpdate`
  (if (`self.IsSelected`)
    (`/Game/Blueprints/BuildingsAndProps/Interactable_Interface.Highlight`)
    (else
      (set `self.IsUsing` false)
      (if (`self.IsHighlighted`)
        (set `self.IsHighlighted` false)
        (else
          (`/Game/Blueprints/BuildingsAndProps/Interactable_Interface.Highlight_Back`))))))

(fn `OnRep_IsDropped`)

(fn `SelectStateUpdate`
  (bind _overlappingactors (`PrimitiveComponent.GetOverlappingActors` (`self.ToPlayerGrabCollision`) "/Game/Blueprints/Octopus/BP_MotionControllerMain.BP_MotionControllerMain_C"))
  (set `self.IsSelected` false)
  (if (> (`KismetArrayLibrary.Array_Length` _overlappingactors) 0)
    (for _array_element _overlappingactors
      (bind _asbp_motion_controller_main (cast `/Game/Blueprints/Octopus/BP_MotionControllerMain` _array_element))
      (if (== (`/Game/Blueprints/Octopus/BP_MotionControllerMain.GripActor` _asbp_motion_controller_main) self)
        (set `self.IsSelected` true)))))

(fn `UserConstructionScript`
  (bind _asbp_gi (cast `/Game/Blueprints/Public/BP_GI` (`GameplayStatics.GetGameInstance`)))
  (set `self.SelectedColor` (`/Game/Blueprints/Public/BP_GI.OctoHighlightColor` _asbp_gi))
  (set `self.UsingColor` (`/Game/Blueprints/Public/BP_GI.OctoUsingColor` _asbp_gi)))