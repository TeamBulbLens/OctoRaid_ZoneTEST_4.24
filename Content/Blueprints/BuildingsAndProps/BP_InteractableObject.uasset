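; Base VR interactable prop that tints its static mesh when a motion controller targets it for gripping.
; Each tick it checks controllers overlapping its Box and marks itself selected if one's GripActor is this actor.
; While selected, it sets the HighlightColor material parameter to a selected or in-use color, both read from BP_GI in the construction script.
; Deselection clears IsUsing and resets the color to black after a one-tick delay.
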(event `self.Highlight`
  ;[1 1 1] highlight
  (cast `/Game/Blueprints/Octopus/BP_VRPawnMain` (`GameplayStatics.GetPlayerPawn` 0))
  (`MeshComponent.SetVectorParameterValueOnMaterials` (`self.StaticMesh`) "HighlightColor" (select `bool` (`self.IsUsing`) :`false` (`KismetMathLibrary.Conv_LinearColorToVector` (`self.SelectedColor`)) :`true` (`KismetMathLibrary.Conv_LinearColorToVector` (`self.UsingColor`))))
  (set `self.IsHighlighted` true))

(event `self.Highlight_Back`
  ;[1 1 1] highlight
  (cast `/Game/Blueprints/Octopus/BP_VRPawnMain` (`GameplayStatics.GetPlayerPawn` 0))
  (`MeshComponent.SetVectorParameterValueOnMaterials` (`self.StaticMesh`) "HighlightColor" (0.0 0.0 0.0)))

(event `self.ReceiveTick`
  (params (DeltaSeconds :type "Float (single-precision)"))
  (bind _overlappingactors (`PrimitiveComponent.GetOverlappingActors` (`self.Box`) "/Game/Blueprints/Octopus/BP_MotionControllerMain.BP_MotionControllerMain_C"))
  ;[1 1 1] 컨트롤러가 잡으려고 할 때 하이라이트 / 아니면 원래대로
  (`|ExecutionSequence`
    (:`then_0`
      (set `self.IsSelected` false)
      (if (> (`KismetArrayLibrary.Array_Length` _overlappingactors) 0)
        (for _array_element _overlappingactors
          (bind _asbp_motion_controller_main (cast `/Game/Blueprints/Octopus/BP_MotionControllerMain` _array_element))
          (if (== (`/Game/Blueprints/Octopus/BP_MotionControllerMain.GripActor` _asbp_motion_controller_main) self)
            (set `self.IsSelected` true)))))
    (:`then_1`
      (if (`self.IsSelected`)
        (`self.Highlight`)
        (else
          (set `self.IsUsing` false)
          (if (`self.IsHighlighted`)
            (set `self.IsHighlighted` false)
            (else
              (`self.Highlight_Back`))))))))

(fn `UserConstructionScript`
  (bind _asbp_gi (cast `/Game/Blueprints/Public/BP_GI` (`GameplayStatics.GetGameInstance`)))
  (set `self.SelectedColor` (`/Game/Blueprints/Public/BP_GI.OctoHighlightColor` _asbp_gi))
  (set `self.UsingColor` (`/Game/Blueprints/Public/BP_GI.OctoUsingColor` _asbp_gi)))