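; Physics prop that can be picked up, carried and then dropped or thrown.
; Pickup turns off Box physics and attaches the root to a given component, with IsUsing blocking repeat pickups.
; Drop re-enables physics, detaches the actor and, when fired, adds linear and angular velocity.
; Tick calls Drop whenever it is unused but has a valid parent component; the IsDropped rep-notify is empty.
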(event `self.Pickup`
  (params (AttachTo :type "SceneComponent Object Reference"))
  ;[1 1 1] Pickup
  (if (not (`self.IsUsing`))
    (`PrimitiveComponent.SetSimulatePhysics` (`self.Box`) false)
    (`SceneComponent.K2_AttachToComponent` (`self.RootComponent`) AttachTo "None" "KeepWorld" "KeepWorld" "KeepWorld" false)
    (set `self.IsUsing` true)))

(event `self.Drop`
  (params (Hand :type "SceneComponent Object Reference") (LinearVelocity :type "Vector Structure") (AngularVelocity :type "Vector Structure") (Fire :type Boolean))
  (bind _box (`self.Box`))
  ;[1 1 1] Pickup
  (`PrimitiveComponent.SetSimulatePhysics` (`self.Box`) true)
  (if Fire
    (`PrimitiveComponent.SetPhysicsLinearVelocity` _box LinearVelocity true "None")
    (`PrimitiveComponent.SetPhysicsAngularVelocityInDegrees` _box AngularVelocity true "None"))
  (`self.K2_DetachFromActor` "KeepWorld" "KeepWorld" "KeepWorld")
  (set `self.IsDropped` true)
  (set `self.IsUsing` false))

(event `self.ReceiveTick`
  (params (DeltaSeconds :type "Float (single-precision)"))
  ;[1 1 1] Tick
  (`parent.ReceiveTick` DeltaSeconds)
  (if (not (`self.IsUsing`))
    (`/Engine/EditorBlueprintResources/StandardMacros.IsValid` (`self.GetParentComponent`)
      (:`Is Valid`
        (`self.Drop` null)))))

(fn `OnRep_IsDropped`)

(fn `UserConstructionScript`)