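; Hunter item spawner that repeatedly spawns a configured item class at the transform of Item1's owner while spawning is switched on.
; Tick, throttled to the respawn delay, waits that delay again, then calls a spawn event that only spawns on authority.
; Actors without the BP_Hunter_Item tag pause spawning and ticking on entering the sphere, and re-enable both when their actor overlap ends.
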(event `self.ReceiveBeginPlay`
  (`self.SetActorTickInterval` (`self.RespawnDelay`)))

(event `self.ReceiveTick`
  (params (DeltaSeconds :type "Float (single-precision)"))
  ;[1 1 1] Item Spawn
  (if (`self.IsSpawn?`)
    (`KismetSystemLibrary.Delay` (`self.RespawnDelay`))
    (`self.ServerSpawnItem`)))

(event `ServerSpawnItem`
  ;[1 1 1] Item Spawn
  (`/Engine/EditorBlueprintResources/ActorMacros.Switch Has Authority`
    (:`Authority`
      (`self.Respawn`))))

(event `self.ReceiveActorEndOverlap`
  (params (OtherActor :type "Actor Object Reference"))
  ;[1 1 1] Spawn Switch
  (if (not (`self.ActorHasTag` OtherActor "BP_Hunter_Item"))
    (set `self.IsSpawn?` true)
    (`self.SetActorTickEnabled` true)))

(event `self.Sphere.OnComponentBeginOverlap`
  (params (OverlappedComponent :type "PrimitiveComponent Object Reference") (OtherActor :type "Actor Object Reference") (OtherComp :type "PrimitiveComponent Object Reference") (OtherBodyIndex :type Integer) (bFromSweep :type Boolean) (SweepResult :type "HitResult Structure (by ref)"))
  ;[1 1 1] Spawn Switch
  (if (not (`self.ActorHasTag` OtherActor "BP_Hunter_Item"))
    (set `self.IsSpawn?` false)
    (`self.SetActorTickEnabled` false)))

(fn `Respawn`
  (`|SpawnActorFromClass` (`self.ItemToLoad`) (`self.GetTransform` (`ActorComponent.GetOwner` (`self.Item_1`))) "Undefined" "OverrideRootScale" null null))

(fn `UserConstructionScript`)