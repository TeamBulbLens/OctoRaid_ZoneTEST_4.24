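; Base Blueprint for a pickup object that explodes once dropped, ignoring motion controller contact.
; An overlap or a hard enough hit on its Box triggers Destruction and ExplosionDamage, which applies radial damage using GameInstance settings.
; Destruction disables physics and collision, hides the mesh, spawns the effect, and destroys the actor after a delay.
; It also plays sound through a server-to-multicast event chain and calls DropItem, an empty hook here.
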(event `self.ReceiveBeginPlay`
  (`parent.ReceiveBeginPlay`)
  (bind _asbp_gi (cast `/Game/Blueprints/Public/BP_GI` (`GameplayStatics.GetGameInstance`)))
  (if (`/Game/Blueprints/Public/BP_GI.IsDebugMode` _asbp_gi)
    _))

(event `self.Box.OnComponentHit`
  (params (HitComponent :type "PrimitiveComponent Object Reference") (OtherActor :type "Actor Object Reference") (OtherComp :type "PrimitiveComponent Object Reference") (NormalImpulse :type "Vector Structure") (Hit :type "HitResult Structure (by ref)"))
  ;[1 1 1] 일정 이상의 충격이 가해지면 부서짐
  (if (`self.IsDropped`)
    (cast `/Game/Blueprints/Octopus/BP_MotionControllerMain` OtherActor
      (:`CastFailed`
        (`/Engine/EditorBlueprintResources/StandardMacros.IsValid` (`GameplayStatics.GetGameMode`)
          (:`Is Valid`
            (if (> (`KismetMathLibrary.VSize` NormalImpulse) 700000.0)
              (`self.Destruction`)
              (`self.ExplosionDamage`))))))))

(event `self.Box.OnComponentBeginOverlap`
  (params (OverlappedComponent :type "PrimitiveComponent Object Reference") (OtherActor :type "Actor Object Reference") (OtherComp :type "PrimitiveComponent Object Reference") (OtherBodyIndex :type Integer) (bFromSweep :type Boolean) (SweepResult :type "HitResult Structure (by ref)"))
  ;[1 1 1] 일정 이상의 충격이 가해지면 부서짐
  (if (`self.IsDropped`)
    (cast `/Game/Blueprints/Octopus/BP_MotionControllerMain` OtherActor
      (:`CastFailed`
        (`/Engine/EditorBlueprintResources/StandardMacros.IsValid` (`GameplayStatics.GetGameMode`)
          (:`Is Valid`
            (`self.Destruction`)
            (`self.ExplosionDamage`)))))))

(event `Destruction`
  (bind (_returnvalue_location _returnvalue_rotation) (`KismetMathLibrary.BreakTransform` (`self.GetTransform`)))
  ;[1 1 1] 부서짐 효과
  (`PrimitiveComponent.SetSimulatePhysics` (`self.Box`) false)
  (`PrimitiveComponent.SetCollisionEnabled` (`self.Box`) "NoCollision")
  (`SceneComponent.SetVisibility` (`self.StaticMesh`) false true)
  (`GameplayStatics.SpawnEmitterAtLocation` (`self.ExplosionEffect`) _returnvalue_location _returnvalue_rotation (`self.Scale`))
  (`self.PlaySound`)
  (`self.DropItem`)
  (`KismetSystemLibrary.Delay` 2.0)
  (`self.K2_DestroyActor`))

(event `DropItem`)

(event `PlaySound`
  (bind (_returnvalue_location _returnvalue_rotation) (`KismetMathLibrary.BreakTransform` (`self.GetTransform`)))
  ;[1 1 1] 폭발음
  (`self.ServerSound` _returnvalue_location))

(event `ServerSound`
  (params (SoundLocation :type "Vector Structure"))
  ;[1 1 1] 폭발음
  (`self.MulticastSound` SoundLocation))

(event `MulticastSound`
  (params (SoundLocation :type "Vector Structure"))
  ;[1 1 1] 폭발음
  (`GameplayStatics.SpawnSoundAtLocation` "/Game/Resources/Ultimate_SFX_Bundle/Warfare_SFX_Bundle/Explosion_Sounds_Pro/Cues/Explosion.Explosion" SoundLocation (struct) 1.0 1.0 0.0 null null))

(fn `ExplosionDamage`
  (bind _asbp_gi (cast `/Game/Blueprints/Public/BP_GI` (`GameplayStatics.GetGameInstance`)))
  (`GameplayStatics.ApplyRadialDamage` :`BaseDamage` (`/Game/Blueprints/Public/BP_GI.ExplosionDamage` _asbp_gi) :`Origin` (`self.K2_GetActorLocation`) :`DamageRadius` (`self.DamageRadius`) :`DamageTypeClass` "/Game/Blueprints/Octopus/DamageType_Object.DamageType_Object_C" :`DamageCauser` null :`InstigatedByController` null :`bDoFullDamage` (`/Game/Blueprints/Public/BP_GI.IsExplosionFullDamage` _asbp_gi)))

(fn `UserConstructionScript`
  (`parent.UserConstructionScript`))