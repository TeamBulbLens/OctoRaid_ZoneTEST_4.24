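; BP_Panel is a double-sided neon screen panel prop with independently configurable front and back faces.
; The construction script creates dynamic instances of M_Panel for the front and back screen meshes.
; It feeds per-side variables into each instance for textures, background color, emissive, hue, desaturation, panner values and UV tiling.
; The event graph has no active logic, so all setup happens at construction.
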(fn `UserConstructionScript`
  (bind _mi_screen_back (`self.MI_Screen_Back`))
  (bind _mi_screen_back_2 (`self.MI_Screen_Back`))
  (bind _mi_screen_back_3 (`self.MI_Screen_Back`))
  (bind _mi_screen_back_4 (`self.MI_Screen_Back`))
  (bind _mi_screen_front (`self.MI_Screen_Front`))
  (bind _mi_screen_front_2 (`self.MI_Screen_Front`))
  (bind _mi_screen_front_3 (`self.MI_Screen_Front`))
  (bind _mi_screen_front_4 (`self.MI_Screen_Front`))
  (bind _returnvalue (`PrimitiveComponent.CreateDynamicMaterialInstance` (`self.SM_Screen_Front`) 0 "/Game/AssetContents/Neon_Materials/Materials/M_Panel/M_Panel.M_Panel" "MI_Screen_Front"))
  (set `self.MI_Screen_Front` _returnvalue)
  (bind _returnvalue_2 (`PrimitiveComponent.CreateDynamicMaterialInstance` (`self.SM_Screen_Back`) 0 "/Game/AssetContents/Neon_Materials/Materials/M_Panel/M_Panel.M_Panel" "MI_Screen_Back"))
  (set `self.MI_Screen_Back` _returnvalue_2)
  (`|ExecutionSequence`
    (:`then_0`
      ;[1 1 1 1 28] Front Textures
      (`MaterialInstanceDynamic.SetTextureParameterValue` _mi_screen_front_2 "Opacity Map" (`self.Opacity Map Front`))
      (`MaterialInstanceDynamic.SetTextureParameterValue` _mi_screen_front_2 "Base Color Map" (`self.Base Color Front`))
      (`MaterialInstanceDynamic.SetTextureParameterValue` _mi_screen_front_2 "Pixel Map" (`self.Pixel Map Front`))
      ;[1 1 1 1 28] Back Textures
      (`MaterialInstanceDynamic.SetTextureParameterValue` _mi_screen_back "Opacity Map" (`self.Opacity Map Back`))
      (`MaterialInstanceDynamic.SetTextureParameterValue` _mi_screen_back "Base Color Map" (`self.Base Color Back`))
      (`MaterialInstanceDynamic.SetTextureParameterValue` _mi_screen_back "Pixel Map" (`self.Pixel Map Back`)))
    (:`then_1`
      ;[1 1 1 1 28] Front Color and Emissive
      (`MaterialInstanceDynamic.SetVectorParameterValue` _mi_screen_front_3 "Background Color" (`self.Background Color Front`))
      (`MaterialInstanceDynamic.SetScalarParameterValue` _mi_screen_front_3 "Emissive" (`self.Emissive Front`))
      (`MaterialInstanceDynamic.SetScalarParameterValue` _mi_screen_front_3 "Desaturation" (`self.Desaturation Front`))
      (`MaterialInstanceDynamic.SetScalarParameterValue` _mi_screen_front_3 "Hue" (`self.Hue Front`))
      ;[1 1 1 1 28] Back Color and Emissive
      (`MaterialInstanceDynamic.SetVectorParameterValue` _mi_screen_back_3 "Background Color" (`self.Background Color Back`))
      (`MaterialInstanceDynamic.SetScalarParameterValue` _mi_screen_back_3 "Emissive" (`self.Emissive Back`))
      (`MaterialInstanceDynamic.SetScalarParameterValue` _mi_screen_back_3 "Desaturation" (`self.Desaturation Back`))
      (`MaterialInstanceDynamic.SetScalarParameterValue` _mi_screen_back_3 "Hue" (`self.Hue Back`)))
    (:`then_2`
      ;[1 1 1 1 28] Front Panners
      (`MaterialInstanceDynamic.SetScalarParameterValue` _mi_screen_front_4 "X Panner" (`self.X_Panner Front`))
      (`MaterialInstanceDynamic.SetScalarParameterValue` _mi_screen_front_4 "Y Panner" (`self.Y_Panner Front`))
      ;[1 1 1 1 28] Back Panners
      (`MaterialInstanceDynamic.SetScalarParameterValue` _mi_screen_back_2 "X Panner" (`self.X_Panner Back`))
      (`MaterialInstanceDynamic.SetScalarParameterValue` _mi_screen_back_2 "Y Panner" (`self.Y_Panner Back`)))
    (:`then_3`
      ;[1 1 1 1 28] Front UV Tiling
      (`MaterialInstanceDynamic.SetScalarParameterValue` _mi_screen_front "U Tiling" (`self.U Tiling Front`))
      (`MaterialInstanceDynamic.SetScalarParameterValue` _mi_screen_front "V Tiling" (`self.V Tiling Front`))
      ;[1 1 1] Comment
      (`MaterialInstanceDynamic.SetScalarParameterValue` _mi_screen_back_4 "U Tiling" (`self.U Tiling Back`))
      (`MaterialInstanceDynamic.SetScalarParameterValue` _mi_screen_back_4 "V Tiling" (`self.V Tiling Back`)))))