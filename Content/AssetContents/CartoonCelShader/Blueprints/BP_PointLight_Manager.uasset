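; Manager actor that feeds scene point lights into the MPC_PointLight material parameter collection, apparently for a cartoon cel shader.
; Every tick it gathers all PointLights, removing hidden or camera-distant ones through a reverse-loop macro.
; Up to 25 remaining lights write position, radius, color and intensity into numbered vector parameters; larger counts skip this write.
; Cull distance and falloff reach the collection on construction and BeginPlay.
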(event `self.ReceiveBeginPlay`
  (`KismetMaterialLibrary.SetScalarParameterValue` "/Game/AssetContents/CartoonCelShader/Materials/MaterialCollections/MPC_PointLight.MPC_PointLight" "Scalar" (`self.Cull Distance`))
  (`KismetMaterialLibrary.SetScalarParameterValue` "/Game/AssetContents/CartoonCelShader/Materials/MaterialCollections/MPC_PointLight.MPC_PointLight" "Scalar1" (`self.Cull Falloff`)))

(event `self.ReceiveTick`
  (params (DeltaSeconds :type "Float (single-precision)"))
  (`self.Initialize Point Lights`)
  (`self.Process Point Lights`))

(fn `Initialize Point Lights`
  (bind _outactors (`GameplayStatics.GetAllActorsOfClass` "/Script/Engine.PointLight"))
  (bind _output_get (set `self.PointLights` _outactors))
  (bind (_array_element _array_index) (`self.Reverse For Each Loop` _output_get)
    (:`Loop Body`
      (bind _pointlightcomponent (`PointLight.PointLightComponent` _array_element))
      (if (not (and (> (`self.Cull Distance`) (`KismetMathLibrary.Vector_Distance` (`SceneComponent.K2_GetComponentLocation` _pointlightcomponent) (`PlayerCameraManager.GetCameraLocation` (`PlayerController.PlayerCameraManager` (`GameplayStatics.GetPlayerController` 0))))) (`SceneComponent.IsVisible` _pointlightcomponent)))
        (`KismetArrayLibrary.Array_Remove` (`self.PointLights`) _array_index)
        (`self.Reset Point Lights `)))))

(fn `Process Point Lights`
  (bind _pointlights (`self.PointLights`))
  (if (> (`KismetArrayLibrary.Array_Length` _pointlights) 25)
    (`KismetMaterialLibrary.SetVectorParameterValue` "/Game/AssetContents/CartoonCelShader/Materials/MaterialCollections/MPC_PointLight.MPC_PointLight" "Vector" (make `LinearColor` 0.0))
    (else
      (for (_array_element _array_index) _pointlights
        (bind _pointlightcomponent (`PointLight.PointLightComponent` _array_element))
        (bind (_returnvalue_x _returnvalue_y _returnvalue_z) (`KismetMathLibrary.BreakVector` (`SceneComponent.K2_GetComponentLocation` _pointlightcomponent)))
        (bind _pointlightcomponent_2 (`PointLight.PointLightComponent` _array_element))
        (`KismetMaterialLibrary.SetVectorParameterValue` "/Game/AssetContents/CartoonCelShader/Materials/MaterialCollections/MPC_PointLight.MPC_PointLight" (`KismetStringLibrary.Conv_StringToName` (`KismetStringLibrary.Concat_StrStr` "Vector" (`KismetStringLibrary.Conv_IntToString` (+ _array_index 1)))) (make `LinearColor` _returnvalue_x _returnvalue_y _returnvalue_z (`LocalLightComponent.AttenuationRadius` _pointlightcomponent_2)))
        (bind (_returnvalue_r _returnvalue_g _returnvalue_b) (break `LinearColor` (`LightComponentBase.GetLightColor` _pointlightcomponent)))
        (`KismetMaterialLibrary.SetVectorParameterValue` "/Game/AssetContents/CartoonCelShader/Materials/MaterialCollections/MPC_PointLight.MPC_PointLight" (`KismetStringLibrary.Conv_StringToName` (`KismetStringLibrary.Concat_StrStr` "Vector" (`KismetStringLibrary.Conv_IntToString` (+ _array_index 26)))) (make `LinearColor` _returnvalue_r _returnvalue_g _returnvalue_b (`LightComponentBase.Intensity` _pointlightcomponent_2)))))))

(fn `Reset Point Lights `
  (bind _linearcolor (make `LinearColor` 0.0))
  (for (_ _array_index) (`self.PointLights`)
    (`KismetMaterialLibrary.SetVectorParameterValue` "/Game/AssetContents/CartoonCelShader/Materials/MaterialCollections/MPC_PointLight.MPC_PointLight" (`KismetStringLibrary.Conv_StringToName` (`KismetStringLibrary.Concat_StrStr` "Vector" (`KismetStringLibrary.Conv_IntToString` (+ _array_index 1)))) _linearcolor)
    (`KismetMaterialLibrary.SetVectorParameterValue` "/Game/AssetContents/CartoonCelShader/Materials/MaterialCollections/MPC_PointLight.MPC_PointLight" (`KismetStringLibrary.Conv_StringToName` (`KismetStringLibrary.Concat_StrStr` "Vector" (`KismetStringLibrary.Conv_IntToString` (+ _array_index 26)))) _linearcolor)))

(fn `UserConstructionScript`
  (`|ExecutionSequence`
    (:`then_0`
      (`self.Reset Point Lights `))
    (:`then_1`
      (`KismetMaterialLibrary.SetScalarParameterValue` "/Game/AssetContents/CartoonCelShader/Materials/MaterialCollections/MPC_PointLight.MPC_PointLight" "Scalar" (`self.Cull Distance`))
      (`KismetMaterialLibrary.SetScalarParameterValue` "/Game/AssetContents/CartoonCelShader/Materials/MaterialCollections/MPC_PointLight.MPC_PointLight" "Scalar1" (`self.Cull Falloff`)))))